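; Blueprint function library of file helpers for reading, writing, deleting and checking files by path.
; Import and export wrap text read and forced save calls, with export also reporting whether the file already existed and was overwritten.
; Delete reads the contents through Import File before removing the file, so it returns the deleted text alongside the success flag.
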(fn `Delete File`
  (params (Path :type String :default "C:\\Users\\"))
  (returns (Success :type Boolean) (`Deleted Text` :type String))
  (locals (String :type String))
  ;[0.9047 0.000304 0.5972] Deletes the file at the given path
  (bind _output_get (set `local.String` (`.Text` (`self.Import File` Path))))
  (bind _returnvalue (`FileHelperBPLibrary.RemoveFile` Path))
  (return _returnvalue _output_get))

(fn `Export File`
  (params (Text :type String) (Path :type String :default "C:\\Users\\"))
  (returns (Success :type Boolean) (Overwrite :type Boolean))
  (locals (Bool :type Boolean))
  ;[0.9387 0 0.6172] Creates or overwrites a file of the given text to the given path
  (bind _output_get (set `local.Bool` (`self.File Exists` Path)))
  (bind (_error _returnvalue) (`FileHelperBPLibrary.SaveText` Path Text false true))
  (return _returnvalue _output_get))

(fn `File Exists`
  (params (Path :type String :default "C:\\Users\\"))
  (returns (Exists :type Boolean))
  ;[0.9823 0 0.6514] Returns whether the given path leads to a file
  (bind _returnvalue (`FileHelperBPLibrary.IsFile` Path))
  (return _returnvalue))

(fn `Import File`
  (params (Path :type String :default "C:\\Users\\"))
  (returns (Success :type Boolean) (Text :type String))
  ;[0.9823 0 0.6445] Reads a file at the given path and returns its content
  (bind (_output _returnvalue) (`FileHelperBPLibrary.ReadText` Path))
  (return _returnvalue _output))